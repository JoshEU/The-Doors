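; Pressure plate Blueprint that resets the level's dummy cube when something overlaps its trigger box.
; On overlap it destroys every existing DummyCube, then, on authority only, spawns a new one at a hard-coded location.
; The same authority branch sets the new cube's material to red, green or blue by matching the current level name to Red_Map, Green_Map or Blue_Map.
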(event `self.BoxtTrigger.OnComponentBeginOverlap`
  (params (OverlappedComponent :type "PrimitiveComponent Object Reference") (OtherActor :type "Actor Object Reference") (OtherComp :type "PrimitiveComponent Object Reference") (OtherBodyIndex :type Integer) (bFromSweep :type Boolean) (SweepResult :type "HitResult Structure (by ref)"))
  ;[1 1 1] When a player overlaps with the pressure plate, check if any dummy cubes exist and destroy them. Then Spawn in a new dummy cube and set its material based on the current level that the players are in
  (bind _outactors (`GameplayStatics.GetAllActorsOfClass` "/Game/MyFolders/Blueprints/DummyCube.DummyCube_C"))
  (for _array_element _outactors
    (`self.K2_DestroyActor` _array_element))
  (`/Engine/EditorBlueprintResources/ActorMacros.Switch Has Authority`
    (:`Authority`
      (bind _returnvalue (`|SpawnActorFromClass` "/Game/MyFolders/Blueprints/DummyCube.DummyCube_C" (`KismetMathLibrary.MakeTransform` (3729.910311 217.228887 400.0)) "Undefined" "MultiplyWithRoot" null null))
      (set `self.DummyCubeRef` _returnvalue)
      (bind _returnvalue_2 (`GameplayStatics.GetCurrentLevelName` true))
      (if (== _returnvalue_2 "Red_Map")
        (`PrimitiveComponent.SetMaterial` (`/Game/MyFolders/Blueprints/DummyCube.Dummy_Cube` (`self.DummyCubeRef`)) 0 "/Game/MyFolders/Materials/Red_Mat.Red_Mat")
        (elif (== "Green_Map" _returnvalue_2)
          (`PrimitiveComponent.SetMaterial` (`/Game/MyFolders/Blueprints/DummyCube.Dummy_Cube` (`self.DummyCubeRef`)) 0 "/Game/MyFolders/Materials/Green_Mat.Green_Mat")
          (elif (== "Blue_Map" _returnvalue_2)
            (`PrimitiveComponent.SetMaterial` (`/Game/MyFolders/Blueprints/DummyCube.Dummy_Cube` (`self.DummyCubeRef`)) 0 "/Game/MyFolders/Materials/Blue_Mat.Blue_Mat")))))))

(fn `UserConstructionScript`)