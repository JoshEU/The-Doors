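; Game mode that tracks the players in the session and triggers a lobby player list refresh whenever one joins or leaves.
; Login and logout add or remove the Mouse_Controller in AllPlayerControllers, then share a single update path.
; After a short delay, that update calls UpdateLobbyPlayerList on BP_GameState to notify the server and clients.
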(event `UpdateLobbyPlayerList`
  ;[1 1 1] Each time a player joins or leaves the lobby, the Server and clients that are in the session are notified
  (`KismetSystemLibrary.Delay` 0.3)
  (bind _asbp_game_state (cast `/Game/MyFolders/Blueprints/BP_GameState` (`GameplayStatics.GetGameState`)))
  (`/Game/MyFolders/Blueprints/BP_GameState.UpdateLobbyPlayerList` _asbp_game_state))

(event `self.K2_PostLogin`
  (params (NewPlayer :type "PlayerController Object Reference"))
  ;[1 1 1] Add or Remove a Player controller from an array containing all Players in the server
  (bind _asmouse_controller (cast `/Game/MyFolders/Blueprints/Mouse_Controller` NewPlayer))
  (`KismetArrayLibrary.Array_Add` (`self.AllPlayerControllers`) _asmouse_controller)
  (`self.UpdateLobbyPlayerList` :!label _label))

(event `self.K2_OnLogout`
  (params (ExitingController :type "Controller Object Reference"))
  ;[1 1 1] Add or Remove a Player controller from an array containing all Players in the server
  (bind _asmouse_controller (cast `/Game/MyFolders/Blueprints/Mouse_Controller` ExitingController))
  (`KismetArrayLibrary.Array_RemoveItem` (`self.AllPlayerControllers`) _asmouse_controller)
  (goto _label))

(fn `UserConstructionScript`)